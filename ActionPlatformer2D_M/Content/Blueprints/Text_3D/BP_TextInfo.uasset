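; BP_TextInfo is a trigger actor that shows an on-screen info text while the player's BP_Captain character stands inside its box.
; When the Captain's capsule component begins overlapping the Box, it creates a WB_InfoText widget for player controller 0, passes it the actor's Text and adds it to the viewport.
; When the capsule leaves the Box, the stored widget is removed from the screen.
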(event `self.ReceiveBeginPlay`)

(event `self.Box.OnComponentBeginOverlap`
  (params (OverlappedComponent :type "PrimitiveComponent Object Reference") (OtherActor :type "Actor Object Reference") (OtherComp :type "PrimitiveComponent Object Reference") (OtherBodyIndex :type Integer) (bFromSweep :type Boolean) (SweepResult :type "HitResult Structure (by ref)"))
  (cast `/Game/Blueprints/Characters/Captain/BP_Captain` OtherActor)
  (cast `CapsuleComponent` OtherComp)
  (bind _returnvalue (`|CreateWidget` "/Game/Blueprints/WB_InfoText.WB_InfoText_C" (`GameplayStatics.GetPlayerController` 0)))
  (bind _output_get (set `self.WidgetBP` _returnvalue))
  (set `/Game/Blueprints/WB_InfoText.InfoText` (`self.Text`) _output_get)
  (`UserWidget.AddToViewport` _output_get 0))

(event `self.Box.OnComponentEndOverlap`
  (params (OverlappedComponent :type "PrimitiveComponent Object Reference") (OtherActor :type "Actor Object Reference") (OtherComp :type "PrimitiveComponent Object Reference") (OtherBodyIndex :type Integer))
  (cast `/Game/Blueprints/Characters/Captain/BP_Captain` OtherActor)
  (cast `CapsuleComponent` OtherComp)
  (`Widget.RemoveFromParent` (`self.WidgetBP`)))

(fn `UserConstructionScript`)